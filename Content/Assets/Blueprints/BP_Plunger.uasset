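; BP_Plunger is a pinball plunger actor that moves on hold and release and launches reactive objects.
; OnHold plays a timeline that lerps the Plunger from start to end position; OnRelease stops it and plays a second timeline back from UpdatedPos to start.
; When an actor stops overlapping the Box, it receives an impulse through BPI_PinballReactive, directed away from the plunger and scaled by MaxForce and ChargeTime.
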(event `OnHold`
  (bind (_direction _0_1) (`Timeline|Timeline` :!via `PlayFromStart` :!label _label)
    (:`Update`
      (`SceneComponent.K2_SetRelativeLocation` (`self.Plunger`) (`KismetMathLibrary.VLerp` (`self.StartPos`) (`self.EndPos`) _0_1) false false))))

(event `OnRelease`
  (`|ExecutionSequence`
    (:`then_0`
      (goto _label :!via `Stop`))
    (:`then_1`
      (bind (_direction _chargealpha) (`Timeline|Timeline02` :!via `PlayFromStart`)
        (:`Update`
          (`SceneComponent.K2_SetRelativeLocation` (`self.Plunger`) (`KismetMathLibrary.VLerp` (`self.UpdatedPos`) (`self.StartPos`) _chargealpha) false false))))))

(event `self.Box.OnComponentEndOverlap`
  (params (OverlappedComponent :type "PrimitiveComponent Object Reference") (OtherActor :type "Actor Object Reference") (OtherComp :type "PrimitiveComponent Object Reference") (OtherBodyIndex :type Integer))
  (bind _asbpi_pinball_reactive (cast `/Game/Assets/BPI_PinballReactive` OtherActor))
  (`/Game/Assets/BPI_PinballReactive.PinballImpulseEvent` _asbpi_pinball_reactive (* (* (`self.MaxForce`) (`self.ChargeTime`)) (`KismetMathLibrary.Normal` (- (`SceneComponent.K2_GetComponentLocation` OtherComp) (`self.K2_GetActorLocation`))))))

(fn `UserConstructionScript`)
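; BP_BallSpawn manages ball spawning and a score value for a ball game with drains.
; On BeginPlay it takes the first TargetPoint found in the level as the spawn point, spawns a BP_Ball there and stores it as the current ball.
; HandleBallDrain spawns a replacement ball at the same point.
; AddScore sets Score to the passed amount, without adding to the previous total, and prints it.
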(event `self.ReceiveBeginPlay`
  (bind _outactors (`GameplayStatics.GetAllActorsOfClass` "/Script/Engine.TargetPoint"))
  (set `self.SpawnPoint` (`|GetArrayItem` _outactors))
  (`self.SpawnBall`))

(fn `AddScore`
  (params (Amount :type Integer))
  (bind _output_get (set `self.Score` (+ Amount 0)))
  (`KismetSystemLibrary.PrintString` (`KismetStringLibrary.Conv_IntToString` _output_get)))

(fn `HandleBallDrain`
  (`self.SpawnBall`))

(fn `SpawnBall`
  (bind _returnvalue (`|SpawnActorFromClass` "/Game/Assets/Blueprints/BP_Ball.BP_Ball_C" (`self.GetTransform` (`self.SpawnPoint`)) "Undefined" "MultiplyWithRoot" null null))
  (set `self.CurrentBall` _returnvalue))

(fn `UserConstructionScript`)
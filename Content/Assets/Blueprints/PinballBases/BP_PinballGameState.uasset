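; Pinball game state that holds the score and the number of balls remaining.
; BeginPlay sets starting values through the SetScore and SetBalls events.
; Each setter stores the new value, calls its OnScoreChanged or OnBallsChanged dispatcher so listeners can react, and prints the value.
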(event `self.ReceiveBeginPlay`
  (`self.SetScore` 100.0)
  (`self.SetBalls` 3))

(event `SetScore`
  (params (NewScore :type "Float (double-precision)"))
  (bind _output_get (set `self.Score` NewScore))
  (`self.OnScoreChanged` _output_get)
  (`KismetSystemLibrary.PrintString` (`KismetStringLibrary.Conv_DoubleToString` _output_get)))

(event `SetBalls`
  (params (NewBalls :type Integer))
  (bind _output_get (set `self.BallsRemaining` NewBalls))
  (`self.OnBallsChanged` _output_get)
  (`KismetSystemLibrary.PrintString` (`KismetStringLibrary.Conv_IntToString` _output_get)))

(fn `UserConstructionScript`)
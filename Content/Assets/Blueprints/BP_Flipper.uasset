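; BP_Flipper is a flipper actor that swings a Flipper component 90 degrees when activated and returns it when deactivated.
; At BeginPlay, the Direction enum picks the sign of the end rotation, so the same Blueprint can swing either way.
; OnActivate plays a timeline that lerps the relative rotation between start and end, and OnDeactivate reverses that timeline from its current position.
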(event `OnActivate`
  (bind (_direction _0_1) (`Timeline|Timeline` :!label _label)
    (:`Update`
      (`SceneComponent.K2_SetRelativeRotation` (`self.Flipper`) (`KismetMathLibrary.RLerp` (`self.StartRot`) (`self.EndRot`) _0_1) false false))))

(event `OnDeactivate`
  (goto _label :!via `Reverse`))

(event `self.ReceiveBeginPlay`
  (bind _output_get (set `self.StartRot` (struct)))
  (set `self.EndRot` (`KismetMathLibrary.ComposeRotators` _output_get (`KismetMathLibrary.SelectRotator` (struct :`Yaw` -90.0) (struct :`Yaw` 90.0) (`|EnumEquality` (`self.Direction`) "NewEnumerator0")))))

(fn `UserConstructionScript`)
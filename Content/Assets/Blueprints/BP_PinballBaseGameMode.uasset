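; Base game mode for a pinball game that spawns the ball at launch and respawns it after a drain.
; On BeginPlay it takes the first TargetPoint in the level as the spawn point and spawns a BP_Ball there, keeping a reference to it as the current ball.
; HandleBallDrain spawns a replacement ball at the same point, with no destruction, life count or scoring handled here.
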(event `self.ReceiveBeginPlay`
  ; Spawn Ball via Target Point
  (bind _outactors (`GameplayStatics.GetAllActorsOfClass` "/Script/Engine.TargetPoint"))
  (set `self.SpawnPoint` (`|GetArrayItem` _outactors))
  (`self.SpawnBall`))

(fn `HandleBallDrain`
  ; Called When Ball Hits Drain
  (`self.SpawnBall`))

(fn `SpawnBall`
  ; Spawn New Ball Upon Game Launch or After Drain
  (bind _returnvalue (`|SpawnActorFromClass` "/Game/Assets/Blueprints/BP_Ball.BP_Ball_C" (`self.GetTransform` (`self.SpawnPoint`)) "Undefined" "MultiplyWithRoot" null null))
  (set `self.CurrentBall` _returnvalue))

(fn `UserConstructionScript`)
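; Scored pinball game mode that tracks score and remaining balls and ends the game when the balls run out.
; AddScore and HandleBallDrain update the mode's own counters and copy them to BP_PinballGameState.
; A drain spawns another ball while any remain; otherwise it shows WBP_GameOver with the game state's score and switches to UI-only input with a visible cursor.
; The HandleBallDrain override does not call its parent implementation.
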(event `self.ReceiveBeginPlay`
  (`parent.ReceiveBeginPlay`))

(fn `AddScore`
  (params (Amount :type Integer))
  (bind _asbp_pinball_game_state (cast `/Game/Assets/Blueprints/PinballBases/BP_PinballGameState` (`GameplayStatics.GetGameState`)))
  (bind _output_get (set `self.Score` (+ Amount (`self.Score`))))
  (`/Game/Assets/Blueprints/PinballBases/BP_PinballGameState.SetScore` _asbp_pinball_game_state (`KismetMathLibrary.Conv_IntToDouble` _output_get)))

(fn `HandleBallDrain`
  (bind _returnvalue (`GameplayStatics.GetPlayerController` 0))
  (bind _asbp_pinball_game_state (cast `/Game/Assets/Blueprints/PinballBases/BP_PinballGameState` (`GameplayStatics.GetGameState`)))
  (bind _output_get (set `self.BallsRemaining` (- (`self.BallsRemaining`) 1)))
  (`/Game/Assets/Blueprints/PinballBases/BP_PinballGameState.SetBalls` _asbp_pinball_game_state _output_get)
  (if (> _output_get 0)
    (`self.SpawnBall`)
    (else
      (bind _returnvalue_2 (`|CreateWidget` "/Game/Assets/Blueprints/WBP_GameOver.WBP_GameOver_C"))
      (bind _output_get_2 (set `self.GameOverUI` _returnvalue_2))
      (`UserWidget.AddToViewport` _output_get_2 0)
      (bind _asbp_pinball_game_state_2 (cast `/Game/Assets/Blueprints/PinballBases/BP_PinballGameState` (`GameplayStatics.GetGameState`)))
      (`/Game/Assets/Blueprints/WBP_GameOver.SetFinalScore` _output_get_2 (`KismetMathLibrary.FTrunc` (`/Game/Assets/Blueprints/PinballBases/BP_PinballGameState.Score` _asbp_pinball_game_state_2)))
      (`WidgetBlueprintLibrary.SetInputMode_UIOnlyEx` _returnvalue null)
      (set `PlayerController.bShowMouseCursor` true _returnvalue))))

(fn `UserConstructionScript`
  (`parent.UserConstructionScript`))